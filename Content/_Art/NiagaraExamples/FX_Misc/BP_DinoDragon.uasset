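; BP_DinoDragon is a Niagara example dino that plays a triangle color burst effect when hit.
; ObjectHit stores the impact point and normal, spawning a pooled system attached to the skeletal mesh root when none is valid and active.
; It passes hit position and normal as Niagara variables, then activates with reset, restarting any active burst.
; GetObjectVelocity returns zero and the construction script is empty.
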(event EventObjectHit
  (params (Impact%20Point :type Vector :default "0, 0, 0") (Impact%20Normal :type Vector :default "0, 0, 0") (Type :type Integer))
  (Variables|Default|SetHit%20Location Impact%20Point)
  (Variables|Default|SetHit%20Normal Impact%20Normal)
  (if (Utilities|IsValid (Variables|Default|GetDino%20Impact))
    (if (Components|Activation|IsActive (Variables|Default|GetDino%20Impact))
      _
      (else
        (bind _returnvalue (Niagara|SpawnSystemAttached "/Game/_Art/NiagaraExamples/FX_SkeletalMesh/NS_Dino_Tris_Color_Burst.NS_Dino_Tris_Color_Burst" (Variables|Default|GetSkeletalMesh) "root" "0, 0, 0" "0, 0, 0" "SnapToTargetIncludingScale" true false "AutoRelease" :!label _label))
        (Variables|Default|SetDino%20Impact _returnvalue)))
    (else
      (goto _label)))
  (Class|NiagaraComponent|SetVariablePosition (Variables|Default|GetDino%20Impact) "HitPosition" (Variables|Default|GetHit%20Location))
  (Niagara|SetNiagaraVariable(Vector3) (Variables|Default|GetDino%20Impact) "HitNormal" (Variables|Default|GetHit%20Normal))
  (Components|Activation|Activate (Variables|Default|GetDino%20Impact) true))

(fn ConstructionScript)

(fn GetObjectVelocity
  (return "0, 0, 0"))