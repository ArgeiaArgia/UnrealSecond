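; BP_FireworkTarget is a target actor in the Niagara examples gallery that sets off a firework burst when hit.
; ObjectHit with Type 1 spawns an auto-released pooled NS_FireworkBurst at the actor and passes its spawn, spread, color and celebration settings as user variables.
; Ring radius follows the root's X scale, and the construction script tints the Boundary effect with BaseColor.
; TriggerFireworks is empty and GetObjectVelocity returns zero.
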(event Custom|TriggerFireworks)

(event EventObjectHit
  (params (Impact%20Point :type Vector :default "0, 0, 0") (Impact%20Normal :type Vector :default "0, 0, 0") (Type :type Integer))
  (if (== Type 1)
    (bind _returnvalue (Niagara|SpawnSystematLocation "/Game/_Art/NiagaraExamples/FX_Misc/NS_FireworkBurst.NS_FireworkBurst" (Transformation|GetActorLocation) (Transformation|GetActorRotation) "1.000000,1.000000,1.000000" true true "AutoRelease"))
    (bind _output_get (Variables|Default|SetNiagara%20System _returnvalue))
    (Niagara|SetNiagaraVariable(Float) _output_get "Spawn Rate" (Variables|Default|GetSpawn%20Rate))
    (Niagara|SetNiagaraVariable(Float) (Variables|Default|GetNiagara%20System) "Spawn Duration Scale" (Variables|Default|GetSpawn%20Duration%20Scale))
    (Niagara|SetNiagaraVariable(Float) (Variables|Default|GetNiagara%20System) "Ring Radius" (* (.X (Math|Vector|BreakVector (Transformation|GetWorldScale (Variables|Default|GetDefaultSceneRoot)))) (Variables|Default|GetTarget%20Radius)))
    (Niagara|SetNiagaraVariable(Float) (Variables|Default|GetNiagara%20System) "Spread" (Variables|Default|GetSpread))
    (Class|NiagaraComponent|SetVariableBool (Variables|Default|GetNiagara%20System) "Enable Burst" (Variables|Default|GetEnable%20Burst))
    (Niagara|SetNiagaraVariable(LinearColor) (Variables|Default|GetNiagara%20System) "Burst Color" (Variables|Default|GetBase%20Color))
    (Class|NiagaraComponent|SetVariableBool (Variables|Default|GetNiagara%20System) "Celebrate" (Variables|Default|GetCelebrate))))

(fn ConstructionScript
  (Niagara|SetNiagaraVariable(LinearColor) (Variables|Default|GetBoundary) "Color" (Variables|Default|GetBase%20Color)))

(fn GetObjectVelocity
  (return "0, 0, 0"))