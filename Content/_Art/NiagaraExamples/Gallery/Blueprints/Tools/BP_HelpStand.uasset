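; BP_HelpStand is a gallery help stand that shows its help text to the player on approach.
; When a BP_Gallery_Character begins overlapping its SphereCollision, it fades in the description on that character's CrosshairWidget using HelpText.
; Ending the overlap fades the description out and clears the text, with validity checks on the widget in both cases.
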(event OnComponentBeginOverlap(SphereCollision)
  (params (OverlappedComponent :type Primitive%20Component%20Object%20Reference) (OtherActor :type Actor%20Object%20Reference) (OtherComp :type Primitive%20Component%20Object%20Reference) (OtherBodyIndex :type Integer) (bFromSweep :type Boolean) (SweepResult :type Hit%20Result%20Structure%20%28by%20ref%29))
  (bind _asbp_gallery_character (Utilities|Casting|CastToBP_Gallery_Character OtherActor))
  (if (Utilities|IsValid (Variables|/Game/_Art/NiagaraExamples/Gallery/Blueprints/BP_Gallery_Character.BP_Gallery_Character_C|GetCrosshair%20Widget _asbp_gallery_character))
    (Default|FadeDescription (Variables|/Game/_Art/NiagaraExamples/Gallery/Blueprints/BP_Gallery_Character.BP_Gallery_Character_C|GetCrosshair%20Widget _asbp_gallery_character) true (Variables|Default|GetHelp%20Text))))

(event OnComponentEndOverlap(SphereCollision)
  (params (OverlappedComponent :type Primitive%20Component%20Object%20Reference) (OtherActor :type Actor%20Object%20Reference) (OtherComp :type Primitive%20Component%20Object%20Reference) (OtherBodyIndex :type Integer))
  (bind _asbp_gallery_character (Utilities|Casting|CastToBP_Gallery_Character OtherActor))
  (if (Utilities|IsValid (Variables|/Game/_Art/NiagaraExamples/Gallery/Blueprints/BP_Gallery_Character.BP_Gallery_Character_C|GetCrosshair%20Widget _asbp_gallery_character))
    (Default|FadeDescription (Variables|/Game/_Art/NiagaraExamples/Gallery/Blueprints/BP_Gallery_Character.BP_Gallery_Character_C|GetCrosshair%20Widget _asbp_gallery_character) false)))

(event EventBeginPlay)

(event Collision|EventActorBeginOverlap
  (params (OtherActor :type Actor%20Object%20Reference)))

(event EventTick
  (params (DeltaSeconds :type Float%20%28single-precision%29)))

(fn ConstructionScript)