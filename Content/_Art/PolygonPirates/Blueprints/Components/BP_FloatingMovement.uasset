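; Component that gives its owning actor a floating sway by rocking its rotation, likely for floating props such as boats.
; It caches the owner's transform at BeginPlay, then each Tick adds sine waves of differing speed and amplitude to roll, pitch and yaw.
; SwayOffset shifts the phase and SwayMultiplier scales the motion.
; Location is reset to the original every frame, so there is no vertical bob.
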(event EventBeginPlay
  (Variables|Default|SetOriginalTransform (Transformation|GetActorTransform (Components|GetOwner))))

(event EventTick
  (params (DeltaSeconds :type Float%20%28single-precision%29))
  (bind _originaltransform (Variables|Default|GetOriginalTransform))
  (bind _swaymultiplier (Variables|Default|GetSwayMultiplier))
  (bind (_x _y _z) (Math|Vector|BreakVector (.location _originaltransform)))
  (bind (_roll _pitch _yaw) (Math|Rotator|BreakRotator (.rotation _originaltransform)))
  (Variables|Default|SetTime (+ DeltaSeconds (Variables|Default|GetTime)))
  (Transformation|SetActorLocationAndRotation (Components|GetOwner) (Math|Vector|MakeVector _x _y _z) (Math|Rotator|MakeRotator (+ _roll (* (Math|Trig|Sin(Degrees) (* (+ (Variables|Default|GetTime) (Variables|Default|GetSwayOffset)) 8e+01)) 3.0 _swaymultiplier)) (+ _pitch (* (Math|Trig|Sin(Degrees) (* (+ (Variables|Default|GetTime) (Variables|Default|GetSwayOffset)) 1e+02)) 5.0 _swaymultiplier)) (+ _yaw (* (Math|Trig|Sin(Degrees) (* (+ (Variables|Default|GetTime) (Variables|Default|GetSwayOffset)) 2e+01)) 4.0 _swaymultiplier)))))